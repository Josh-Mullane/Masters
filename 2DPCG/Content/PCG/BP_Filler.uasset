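; BP_Filler is a procedural-generation filler piece that picks its Paper2D tile map on BeginPlay.
; When OldZ and NewZ differ, it uses the down map if NewZ is higher, otherwise the up map, which it also raises along Z by a fixed offset.
; When the heights match, it picks a random map from FillerArray using the Seed random stream.
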(event EventBeginPlay
  (bind _papertilemap (Variables|Default|GetPaperTileMap))
  (bind _newz (Variables|Default|GetNewZ))
  (bind _oldz (Variables|Default|GetOldZ))
  (bind _papertilemap_2 (Variables|Default|GetPaperTileMap))
  (bind _returnvalue (Transformation|GetWorldLocation _papertilemap_2))
  (bind _returnvalue_2 (> _newz _oldz))
  (if (!= (Variables|Default|GetOldZ) (Variables|Default|GetNewZ))
    (Class|PaperTileMapComponent|SetTileMap _papertilemap (select _returnvalue_2 "/Game/PCG/TileMaps/Fillers/TM_FillerDown.TM_FillerDown" "/Game/PCG/TileMaps/Fillers/TM_FillerUp.TM_FillerUp"))
    (if (not _returnvalue_2)
      (Transformation|SetWorldLocation (Variables|Default|GetPaperTileMap) (Math|Vector|MakeVector (.x _returnvalue) (.y _returnvalue) (+ (.z _returnvalue) 1.6e+02)) false false))
    (else
      (Class|PaperTileMapComponent|SetTileMap _papertilemap (.OutItem (Utilities|Array|RandomFromStream (Variables|Default|GetFillerArray) (Variables|Default|GetSeed)))))))

(fn ConstructionScript)