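; BP_Spawner procedurally builds a 2D level by recursively spawning copies of itself, each showing a random tilemap room, up to MaxRooms.
; The middle path advances at fixed intervals and launches a top path that climbs, flattens, then descends using the saved climb angle.
; BP_Filler tiles bridge room gaps, stepping height on a 160-unit grid.
; The last middle room messages overlapping actors to stop, and difficulty is only displayed as text.
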(event EventSTOP
  (Variables|Default|SetSTOP? true)
  (if (Utilities|Enum|Equal(Enum) (Variables|Default|GetPath) "TOP")
    (Actor|DestroyActor)))

(event EventBeginPlay
  (CallFunction|DetermineDifficulty)
  (if (< (.z (Transformation|GetWorldLocation (Variables|Default|GetArrow))) (.z (Variables|Default|GetInitialCoords)))
    (Actor|DestroyActor)
    (else
      (Class|PaperTileMapComponent|SetTileMap (Variables|Default|GetPaperTileMap) (.OutItem (Utilities|Array|Random (Variables|Default|GetMapArray:Diff0))))
      (if (< (Variables|Default|GetNumber) (Variables|Default|GetMaxRooms))
        (switch string (Variables|Default|GetPath)
          (:TOP
            (bind _transform (CallFunction|ContinueTopPath))
            (CallFunction|TopFiller _transform))
          (:MIDDLE
            (if (< (Variables|Default|GetNumber) 1)
              (CallFunction|RandomiseArrow)
              (CallFunction|SpawnTopPath))
            (bind _spawnloc (CallFunction|SpawnMiddlePath))
            (CallFunction|MiddleFiller _spawnloc)))
        (else
          (Utilities|FlowControl|DelayUntilNextTick)
          (CallFunction|CheckEndCollision))))))

(fn ConstructionScript)

(fn RandomiseArrow
  (bind _returnvalue (Math|Random|RandomFloatinRange 3e+01 6e+01))
  (Variables|Default|SetCurrentAngle _returnvalue)
  (Variables|Default|SetInitialAngle _returnvalue)
  (Transformation|SetWorldRotation (Variables|Default|GetTopArrow) (Math|Rotator|MakeRotator 0.0 _returnvalue 0.0) false false))

(fn SpawnTopPath
  (Game|SpawnActorfromClass "BP_Spawner_C" (Utilities|SpawnTransformTop) "Undefined" "MultiplyWithRoot" 0 (+ (Variables|Default|GetNumber) 1) "TOP" (Variables|Default|GetCurrentAngle) 0.0 0.0 false (Variables|Default|GetInitialCoords) 0))

(fn SpawnMiddlePath
  (bind _interval (Variables|Default|GetInterval))
  (bind _arrow (Variables|Default|GetArrow))
  (bind _returnvalue (Transformation|GetWorldTransform _arrow))
  (bind _returnvalue_2 (Math|Vector|GetForwardVector _arrow))
  (bind _returnvalue_3 (* _returnvalue_2 _interval))
  (bind _returnvalue_4 (+ _returnvalue_3 (.location _returnvalue)))
  (bind _returnvalue_5 (Math|Transform|MakeTransform _returnvalue_4 (.rotation _returnvalue) (.scale _returnvalue)))
  (Game|SpawnActorfromClass "BP_Spawner_C" _returnvalue_5 "Undefined" "MultiplyWithRoot" 0 (+ (Variables|Default|GetNumber) 1) "MIDDLE" 0.0 0.0 0.0 false (Variables|Default|GetInitialCoords) 0)
  (return _returnvalue_5))

(fn ContinueTopPath
  (bind _number (Variables|Default|GetNumber))
  (bind _maxrooms (Variables|Default|GetMaxRooms))
  (bind _returnvalue (/ _maxrooms 2))
  (bind _returnvalue_2 (> _number _returnvalue))
  (if _returnvalue_2
    (bind _transform (CallFunction|TopSecondHalf))
    (else
      (bind _transform_2 (CallFunction|TopFirstHalf))))
  (return (select _returnvalue_2 _transform _transform_2)))

(fn TopFirstHalf
  (bind _returnvalue (Utilities|SpawnTransformTop))
  (bind _currentangle (Variables|Default|GetCurrentAngle))
  (bind _returnvalue_2 (/ _currentangle 2.0))
  (bind _returnvalue_3 (< _returnvalue_2 1e+01))
  ;[0.15 0.15 0.15 0.5] If the current angle is less than 10 degrees, which will happen quickly, it will remember that final angle to mirror the descent of the top path with the ascent. AND is necessary to not override this when the value snaps to 0
  (if (and (!= _returnvalue_2 0.0) _returnvalue_3)
    (if (== (Variables|Default|GetFinalAngle) 0.0)
      (Variables|Default|SetFinalAngle _currentangle)))
  (Transformation|SetWorldRotation (Variables|Default|GetTopArrow) (Math|Rotator|MakeRotator 0.0 (select _returnvalue_3 0.0 _returnvalue_2) 0.0) false false)
  (Game|SpawnActorfromClass "BP_Spawner_C" _returnvalue "Undefined" "MultiplyWithRoot" 0 (+ (Variables|Default|GetNumber) 1) "TOP" _returnvalue_2 (Variables|Default|GetInitialAngle) (Variables|Default|GetFinalAngle) false (Variables|Default|GetInitialCoords) 0)
  (return _returnvalue))

(fn TopSecondHalf
  (bind _returnvalue (Utilities|SpawnTransformTop))
  (if (Variables|Default|GetSTOP?)
    (Actor|DestroyActor)
    (else
      ;[0.15 0.15 0.15 0.5] Easiest way to only use the "final angle" variable once
      (if (Variables|Default|GetDownStarted?)
        _
        (else
          (Variables|Default|SetCurrentAngle (* (Variables|Default|GetFinalAngle) -1.0))))
      (Transformation|SetWorldRotation (Variables|Default|GetTopArrow) (Math|Rotator|MakeRotator 0.0 (select (Variables|Default|GetDownStarted?) (* (Variables|Default|GetCurrentAngle) 1.3) (Variables|Default|GetCurrentAngle)) 0.0) false false)
      (bind _output_get (Variables|Default|SetDownStarted? true))
      (Game|SpawnActorfromClass "BP_Spawner_C" _returnvalue "Undefined" "MultiplyWithRoot" 0 (+ (Variables|Default|GetNumber) 1) "TOP" (select (Variables|Default|GetDownStarted?) (* (Variables|Default|GetCurrentAngle) 1.3) (Variables|Default|GetCurrentAngle)) 0.0 0.0 _output_get (Variables|Default|GetInitialCoords) 0)
      (return _returnvalue))))

(fn CheckEndCollision
  (if (Utilities|Enum|Equal(Enum) (Variables|Default|GetPath) "MIDDLE")
    ;[0.15 0.15 0.15 0.5] DEBUG DISABLE LATER
    (Rendering|SetVisibility (Variables|Default|GetBox) true false)
    (for _array_element (Collision|GetOverlappingActors (Variables|Default|GetBox) 0 :!class /Script/Engine.PrimitiveComponent)
      (Class|BISpawnerComs|STOP(Message) _array_element))))

(fn DetermineDifficulty
  (bind _returnvalue (Math|Random|RandomBool))
  (bind _number (Variables|Default|GetNumber))
  (bind _prevdifficulty (Variables|Default|GetPrevDifficulty))
  (bind _returnvalue_2 (< _number 2))
  (bind _returnvalue_3 (+ _prevdifficulty 1))
  (bind _returnvalue_4 (- _prevdifficulty 1))
  (bind _returnvalue_5 (> _returnvalue_4 -1))
  (bind _returnvalue_6 (select _returnvalue_5 _returnvalue_4 3))
  (bind _returnvalue_7 (select _returnvalue _returnvalue_3 _returnvalue_6))
  (bind _returnvalue_8 (select _returnvalue_2 0 _returnvalue_7))
  (Rendering|Components|TextRender|SetText (Variables|Default|GetTextRender) (|GenerictoText _returnvalue_8))
  (return _returnvalue_8))

(fn MiddleFiller
  (params (EndLoc :type Transform))
  (Variables|Default|SetCurrentFillNum (.x (.location EndLoc)))
  (bind _mapwidth (Class|PaperTileMapComponent|GetMapSize (Variables|Default|GetPaperTileMap)))
  (for _index (range 0 (- (/ (- (Variables|Default|GetInterval) (* _mapwidth 160)) 160) 1))
    (bind _output_get (Variables|Default|SetCurrentFillNum (- (Variables|Default|GetCurrentFillNum) 1.6e+02)))
    (Game|SpawnActorfromClass "/Game/PCG/BP_Filler.BP_Filler_C" (Math|Transform|MakeTransform (Math|Vector|MakeVector _output_get (.y (.location EndLoc)) (.z (.location EndLoc))) (.rotation EndLoc) (.scale EndLoc)) "Undefined" "MultiplyWithRoot" 0 0.0 0.0 0)))

(fn TopFiller
  (params (EndLoc :type Transform))
  (bind _papertilemap (Variables|Default|GetPaperTileMap))
  (bind _returnvalue (Transformation|GetWorldLocation _papertilemap))
  (Variables|Default|SetCurrentFillNum (.x (.location EndLoc)))
  (bind _mapwidth (Class|PaperTileMapComponent|GetMapSize (Variables|Default|GetPaperTileMap)))
  (LocalVariables|SetStartZ (.z (.location EndLoc)))
  (LocalVariables|SetNewZ (.z (.location EndLoc)))
  (if (!= (.z (.location EndLoc)) (.z _returnvalue))
    (if (> (.z _returnvalue) (.z (.location EndLoc)))
      (LocalVariables|SetHeightIncrements (Math|Float|Truncate (/ (- (.z _returnvalue) (.z (.location EndLoc))) 1.6e+02)))
      (LocalVariables|SetHeightIndex 2)
      (for _index (range 0 (- (/ (- (Variables|Default|GetInterval) (* _mapwidth 160)) 160) 1)) :!label _label
        (LocalVariables|SetStartZ (LocalVariables|GetNewZ))
        (if (!= (LocalVariables|GetHeightIncrements) 0)
          (switch int (LocalVariables|GetHeightIndex)
            (:0
              _)
            (:1
              (LocalVariables|SetNewZ (- (LocalVariables|GetNewZ) 1.6e+02)))
            (:2
              (LocalVariables|SetNewZ (+ (LocalVariables|GetNewZ) 1.6e+02))))
          (Math|Integer|DecrementInt (LocalVariables|GetHeightIncrements)
            (:%20%20
              _)))
        (bind _output_get (Variables|Default|SetCurrentFillNum (- (Variables|Default|GetCurrentFillNum) 1.6e+02)))
        (Game|SpawnActorfromClass "/Game/PCG/BP_Filler.BP_Filler_C" (Math|Transform|MakeTransform (Math|Vector|MakeVector _output_get (.y (.location EndLoc)) (LocalVariables|GetNewZ)) (.rotation EndLoc) (.scale EndLoc)) "Undefined" "MultiplyWithRoot" 0 (LocalVariables|GetStartZ) (LocalVariables|GetNewZ) 0))
      (elif (< (.z _returnvalue) (.z (.location EndLoc)))
        ;[0.15 0.15 0.15 0.5] HEIGHT INDEX KEY - 0 = no height change, 1 = step up, 2 = step down
        (LocalVariables|SetHeightIncrements (Math|Float|Truncate (/ (- (.z (.location EndLoc)) (.z _returnvalue)) 1.6e+02)))
        (LocalVariables|SetHeightIndex 1)
        (goto _label)))
    (else
      (goto _label))))